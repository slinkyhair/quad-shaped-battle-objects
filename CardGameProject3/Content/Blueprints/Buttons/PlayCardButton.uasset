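; PlayCardButton is a clickable 3D button actor that signals a play press in the card battle.
; Clicking its static mesh plays a press sound and calls PlayButtonPressed on the BattleCardGameState.
; It then fakes a physical press by nudging the whole actor down and, after a brief delay, back up.
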(event `self.StaticMeshComponent.OnClicked`
  (params (TouchedComponent :type "PrimitiveComponent Object Reference") (ButtonPressed :type "Key Structure" :default "AnyKey"))
  (`GameplayStatics.PlaySound2D` "/Game/Sounds/Button_Press_Cue.Button_Press_Cue")
  (bind _asbattle_card_game_state (cast `/Game/Blueprints/BattleCardGameState` (`GameplayStatics.GetGameState`)))
  (`/Game/Blueprints/BattleCardGameState.PlayButtonPressed` _asbattle_card_game_state)
  (`self.K2_SetActorRelativeLocation` (+ (`self.K2_GetActorLocation`) (0.0 0.0 -2.0)))
  (`KismetSystemLibrary.Delay` 0.09)
  (`self.K2_SetActorRelativeLocation` (+ (`self.K2_GetActorLocation`) (0.0 0.0 2.0))))

(fn `UserConstructionScript`)