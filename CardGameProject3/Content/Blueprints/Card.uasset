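; Card actor for a battle card game that loads its stats by ID from the CardDatabase data table and shows them on text components.
; Effect descriptions are generated from type and value, with negative values meaning per-turn effects for some types.
; Timelines lerp movement and rotation.
; Clicks, gated by the game state's active-card check, either report a hand card to BattleCardGameState or remove and destroy a board card.
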(event `ModifyText`
  (params (ID :type Integer))
  ;[1 1 1] Modify Text
  (bind _returnvalue (`|GetDataTableRow` "/Game/Data/CardDatabase.CardDatabase" (`KismetStringLibrary.Conv_StringToName` (`KismetStringLibrary.Conv_IntToString` ID)))
    (:`then`
      (set `self.CardData` _returnvalue)
      (bind (_cardid _name _cost _iscreature _power _cardeffect _effectvalue _dealscombatdamage _hastargetedability) (break `/Game/Data/CardDataStruct` _returnvalue))
      (`self.SetCardText` _name _cost _iscreature _power _cardeffect _effectvalue _dealscombatdamage _hastargetedability))))

(event `move`
  (params (target :type "Vector Structure"))
  ;[1 1 1] handle simple movement
  (set `self.worldLocation` (`self.K2_GetActorLocation`))
  (set `self.endLocation` target)
  (bind (_direction _alpha) (`Timeline|Timeline_0` :!via `PlayFromStart`)
    (:`Update`
      (`self.K2_SetActorRelativeLocation` (`KismetMathLibrary.VLerp` (`self.worldLocation`) (`self.endLocation`) _alpha)))))

(event `rotate`
  (params (target :type "Rotator Structure"))
  ;[1 1 1] handle simple rotation
  (set `self.worldRotator` (`self.K2_GetActorRotation`))
  (set `self.endRotator` target)
  (bind (_direction _alpha) (`Timeline|Timeline_1` :!via `PlayFromStart`)
    (:`Update`
      (`self.K2_SetActorRelativeRotation` (`KismetMathLibrary.RLerp` (`self.worldRotator`) (`self.endRotator`) _alpha)))))

(event `self.StaticMeshComponent.OnClicked`
  (params (TouchedComponent :type "PrimitiveComponent Object Reference") (ButtonPressed :type "Key Structure" :default "AnyKey"))
  (bind _index (`self.Index`))
  ;[1 1 1] Handle control of cards being played
  ;;[1 1 1] Check if another card is active that is not this one
  (bind _asbattle_card_game_state (cast `/Game/Blueprints/BattleCardGameState` (`GameplayStatics.GetGameState`)))
  (bind (_active _index_2) (`/Game/Blueprints/BattleCardGameState.ActiveCardCheck` _asbattle_card_game_state))
  (if (or (not _active) (== _index_2 (`self.Index`)))
    (if (`self.InHand`)
      (bind _asbattle_card_game_state_2 (cast `/Game/Blueprints/BattleCardGameState` (`GameplayStatics.GetGameState`)))
      (`/Game/Blueprints/BattleCardGameState.HandCardClicked` _asbattle_card_game_state_2 _index)
      (else
        (bind _asbattle_card_game_state_3 (cast `/Game/Blueprints/BattleCardGameState` (`GameplayStatics.GetGameState`)))
        (`/Game/Blueprints/BattleCardGameState.RemoveFromBoard` _asbattle_card_game_state_3 _index)
        (`self.K2_DestroyActor`)))))

(fn `GetCreatureDescriptionText`
  (params (CardEffect :type "/Game/Data/CardAbility Enum") (EffectValue :type Integer))
  (returns (DescriptionText :type String))
  ;[1 1 1] Handle positive effect value (instant effect)
  (set `self.NormalValue` EffectValue)
  (if (>= (`self.NormalValue`) 0)
    (switch `/Game/Data/CardAbility` CardEffect
      (:`NewEnumerator0`
        (bind _output_get (set `self.varText` ""))
        (return _output_get))
      (:`NewEnumerator1`
        (bind _output_get_2 (set `self.varText` (`KismetStringLibrary.Concat_StrStr` (`KismetStringLibrary.Concat_StrStr` "When summoned<br>Heal " (`KismetStringLibrary.Conv_IntToString` EffectValue)) " health")))
        (return _output_get_2))
      (:`NewEnumerator2`
        (bind _output_get_3 (set `self.varText` (`KismetStringLibrary.Concat_StrStr` "When summoned<br>increase a creature's<br>power by  " (`KismetStringLibrary.Conv_IntToString` EffectValue))))
        (return _output_get_3))
      (:`NewEnumerator3`
        (bind _output_get_4 (set `self.varText` (`KismetStringLibrary.Concat_StrStr` (`KismetStringLibrary.Concat_StrStr` "When summoned<br>Deal " (`KismetStringLibrary.Conv_IntToString` EffectValue)) " damage")))
        (return _output_get_4))
      (:`NewEnumerator4`
        (bind _output_get_5 (set `self.varText` (`KismetStringLibrary.Concat_StrStr` (`KismetStringLibrary.Concat_StrStr` "When summoned<br>Deal " (`KismetStringLibrary.Conv_IntToString` EffectValue)) " damage<br>to opponent")))
        (return _output_get_5))
      (:`NewEnumerator5`
        (bind _output_get_6 (set `self.varText` (`KismetStringLibrary.Concat_StrStr` (`KismetStringLibrary.Concat_StrStr` "When summoned<br>Deal" (`KismetStringLibrary.Conv_IntToString` EffectValue)) " damage<br>to enemy creatures")))
        (return _output_get_6))
      (:`NewEnumerator6`
        (bind _output_get_7 (set `self.varText` (`KismetStringLibrary.Concat_StrStr` (`KismetStringLibrary.Concat_StrStr` "When summoned<br>Draw" (`KismetStringLibrary.Conv_IntToString` EffectValue)) " cards")))
        (return _output_get_7))
      (:`NewEnumerator7`
        (bind _output_get_8 (set `self.varText` (`KismetStringLibrary.Concat_StrStr` (`KismetStringLibrary.Concat_StrStr` "When summoned<br>gainl" (`KismetStringLibrary.Conv_IntToString` EffectValue)) " cards")))
        (return _output_get_8))
      (:`NewEnumerator8`
        (return "Rush<br>(Can attack 1st turn)"))
      (:`NewEnumerator9`
        (return "Resilience<br>(Ignore 1st<br>damage event)"))
      (:`NewEnumerator10`
        (return "Frenzy<br>(Can attack twice<br>per turn)")))
    (else
      ;[1 1 1] Handle negative effect value (persistent effect)
      (bind _output_get_9 (set `self.NormalValue` (* (`self.NormalValue`) -1)))
      (switch `/Game/Data/CardAbility` CardEffect ; If effect value negative
        (:`NewEnumerator0`
          (return ""))
        (:`NewEnumerator1`
          (return ""))
        (:`NewEnumerator2`
          (return ""))
        (:`NewEnumerator3`
          (return ""))
        (:`NewEnumerator4`
          (bind _output_get_10 (set `self.varText` (`KismetStringLibrary.Concat_StrStr` (`KismetStringLibrary.Concat_StrStr` "Deal " (`KismetStringLibrary.Conv_IntToString` _output_get_9)) " damage<br>to opponent<br>every turn")))
          (return _output_get_10))
        (:`NewEnumerator5`
          (bind _output_get_11 (set `self.varText` (`KismetStringLibrary.Concat_StrStr` (`KismetStringLibrary.Concat_StrStr` "Deal " (`KismetStringLibrary.Conv_IntToString` _output_get_9)) " damage<br>to enemy creatures<br>every turn")))
          (return _output_get_11))
        (:`NewEnumerator6`
          (bind _output_get_12 (set `self.varText` (`KismetStringLibrary.Concat_StrStr` (`KismetStringLibrary.Concat_StrStr` "Draw " (`KismetStringLibrary.Conv_IntToString` _output_get_9)) " cards<br>every turn")))
          (return _output_get_12))
        (:`NewEnumerator7`
          (return ""))
        (:`NewEnumerator8`
          (return ""))
        (:`NewEnumerator9`
          (return ""))
        (:`NewEnumerator10`
          (return ""))))))

(fn `GetLocation`
  (returns (Location :type "Vector Structure"))
  (return (`self.K2_GetActorLocation`)))

(fn `GetManaCost`
  (returns (ManaCost :type Integer))
  (return (`.Cost_30_3F84B31349A40FF38CF10FA191405ED6` (break `/Game/Data/CardDataStruct` (`self.CardData`)))))

(fn `moveCard`
  (params (target :type "Vector Structure"))
  (`self.move` target)
  (return))

(fn `rotateCard`
  (params (target :type "Rotator Structure"))
  (`self.rotate` target)
  (return))

(fn `SetCardText`
  (params (Name :type String) (Cost :type Integer) (IsCreature :type Boolean) (Power :type Integer) (CardEffect :type "/Game/Data/CardAbility Enum") (EffectValue :type Integer) (DealsCombatDamage :type Boolean) (HasTargetedEffect :type Boolean))
  (`TextRenderComponent.K2_SetText` (`self.Name`) (`KismetTextLibrary.Conv_StringToText` Name))
  (`TextRenderComponent.K2_SetText` (`self.Cost`) (`KismetTextLibrary.Conv_StringToText` (`KismetStringLibrary.Conv_IntToString` Cost)))
  (if DealsCombatDamage
    (`TextRenderComponent.SetTextRenderColor` (`self.Power`) (make `Color` 0 0 255))
    (else
      (`TextRenderComponent.SetTextRenderColor` (`self.Power`) (make `Color` 150))))
  (`TextRenderComponent.K2_SetText` (`self.Power`) (`KismetTextLibrary.Conv_StringToText` (`KismetStringLibrary.Conv_IntToString` Power)))
  (bind _descriptiontext (`self.GetCreatureDescriptionText` CardEffect EffectValue))
  (`TextRenderComponent.K2_SetText` (`self.Description`) (`KismetTextLibrary.Conv_StringToText` _descriptiontext)))

(fn `SetIndex`
  (params (NewIndex :type Integer))
  (set `self.Index` NewIndex))

(fn `UserConstructionScript`
  (bind _returnvalue (`|GetDataTableRow` "/Game/Data/CardDatabase.CardDatabase" "11")
    (:`then`
      (set `self.CardData` _returnvalue)
      (bind (_cardid _name _cost _iscreature _power _cardeffect _effectvalue _dealscombatdamage _hastargetedability) (break `/Game/Data/CardDataStruct` _returnvalue))
      (`self.SetCardText` _name _cost _iscreature _power _cardeffect _effectvalue _dealscombatdamage _hastargetedability))))