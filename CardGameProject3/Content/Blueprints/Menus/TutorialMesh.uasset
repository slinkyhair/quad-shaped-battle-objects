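; TutorialMesh is a clickable tutorial actor for the card battle, showing the text indexed by the game instance's TutorialCount.
; On BeginPlay it displays the current text, and clicks on its mesh at steps 0, 2 and 4 advance the count and text.
; At steps 1, 3 and 5 it destroys itself, with 1 and 3 incrementing the count and 1 and 5 calling continue functions on BattleCardGameState.
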(event `SetTutorialText`
  (params (TextValue :type Integer))
  (`TextRenderComponent.K2_SetText` (`self.TextRender`) (`KismetSystemLibrary.MakeLiteralText` (`KismetArrayLibrary.Array_Get` (`self.Tutorial Texts`) TextValue))))

(event `self.ReceiveBeginPlay`
  (bind _asbattle_game_instance (cast `/Game/Blueprints/BattleGameInstance` (`GameplayStatics.GetGameInstance`)))
  (`self.SetTutorialText` (`/Game/Blueprints/BattleGameInstance.TutorialCount` _asbattle_game_instance)))

(event `self.StaticMeshComponent.OnClicked`
  (params (TouchedComponent :type "PrimitiveComponent Object Reference") (ButtonPressed :type "Key Structure" :default "AnyKey"))
  (bind _asbattle_game_instance (cast `/Game/Blueprints/BattleGameInstance` (`GameplayStatics.GetGameInstance`)))
  (bind _tutorialcount (`/Game/Blueprints/BattleGameInstance.TutorialCount` _asbattle_game_instance))
  (if (or (== _tutorialcount 0) (== _tutorialcount 2) (== _tutorialcount 4))
    (bind _result (`/Engine/EditorBlueprintResources/StandardMacros.IncrementInt` _tutorialcount)
      (:`  `
        (`self.SetTutorialText` _result)))
    (else
      (switch `int` _tutorialcount
        (:`1`
          (`/Engine/EditorBlueprintResources/StandardMacros.IncrementInt` _tutorialcount
            (:`  `
              (bind _asbattle_card_game_state (cast `/Game/Blueprints/BattleCardGameState` (`GameplayStatics.GetGameState`)))
              (`/Game/Blueprints/BattleCardGameState.ContinueFromTutorial1` _asbattle_card_game_state)
              (`self.K2_DestroyActor`))))
        (:`3`
          (`/Engine/EditorBlueprintResources/StandardMacros.IncrementInt` _tutorialcount
            (:`  `
              (`self.K2_DestroyActor`))))
        (:`5`
          (bind _asbattle_card_game_state_2 (cast `/Game/Blueprints/BattleCardGameState` (`GameplayStatics.GetGameState`)))
          (`/Game/Blueprints/BattleCardGameState.ContinueFromTutorial3` _asbattle_card_game_state_2)
          (`self.K2_DestroyActor`))))))

(fn `UserConstructionScript`)