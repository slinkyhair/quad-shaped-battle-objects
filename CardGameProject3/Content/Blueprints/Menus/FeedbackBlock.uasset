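; FeedbackBlock is a short-lived menu actor that shows a feedback message on a TextRender component.
; DoItsThing starts a two-second self-destruct delay, sets the given text and plays a timeline.
; The timeline's alpha lerps the actor's relative transform from Start to End while the delay runs.
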(event `SetFeedbackText`
  (params (NewText :type Text))
  (`TextRenderComponent.K2_SetText` (`self.TextRender`) NewText))

(event `DoItsThing`
  (params (Text :type Text))
  (`self.DestroyTimer`)
  (`self.SetFeedbackText` Text)
  (bind (_direction _alpha) (`Timeline|Timeline_0`)
    (:`Update`
      (`self.K2_SetActorRelativeTransform` (`KismetMathLibrary.TLerp` (`self.Start`) (`self.End`) _alpha)))))

(event `DestroyTimer`
  (`KismetSystemLibrary.Delay` 2.0)
  (`self.K2_DestroyActor`))

(fn `UserConstructionScript`)