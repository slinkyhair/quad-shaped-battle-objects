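; Game state for a user-versus-AI card battle that spawns both character cards and decks, deals opening hands and tracks hands, boards and mana.
; Gates turn card clicks into zoom, mana-checked play or combat.
; Combat subtracts each card's Power from the other's, destroying depleted non-character cards and re-indexing positions.
; The AI turn attacks the user's character with each board card, attempts hand plays, then returns the turn through BattleCardGameMode.
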(event `SpawnCharacterCards`
  ;[1 1 1] Character Spawning
  (bind _returnvalue (`|SpawnActorFromClass` "/Game/Blueprints/Card.Card_C" (`KismetMathLibrary.MakeTransform` (`self.CharacterLocation1`) (struct :`Yaw` 180.0)) "Undefined" "OverrideRootScale"))
  (bind _output_get (set `self.UserCharacter` _returnvalue))
  (`/Game/Blueprints/Card.InitCharacter` _output_get true)
  (bind _returnvalue_2 (`|SpawnActorFromClass` "/Game/Blueprints/Card.Card_C" (`KismetMathLibrary.MakeTransform` (`self.CharacterLocation2`) (struct :`Yaw` 180.0)) "Undefined" "OverrideRootScale"))
  (bind _output_get_2 (set `self.AICharacter` _returnvalue_2))
  (`/Game/Blueprints/Card.InitCharacter` _output_get_2 false))

(event `self.ReceiveBeginPlay`
  (bind _delayamount (`self.delayAmount`))
  ;[1 1 1] Draw a full hand
  (`self.SpawnCharacterCards`)
  (bind _returnvalue (`|SpawnActorFromClass` "/Game/Blueprints/Deck.Deck_C" (`KismetMathLibrary.MakeTransform` (`self.DeckLocation1`) (`self.DeckRotation1`)) "Undefined" "OverrideRootScale"))
  (bind _output_get (set `self.Deck1` _returnvalue))
  (`/Game/Blueprints/Deck.InitializeDeck` _output_get false)
  (bind _returnvalue_2 (`|SpawnActorFromClass` "/Game/Blueprints/Deck.Deck_C" (`KismetMathLibrary.MakeTransform` (`self.DeckLocation2`) (`self.DeckRotation1`)) "Undefined" "OverrideRootScale"))
  (bind _output_get_2 (set `self.Deck2` _returnvalue_2))
  (`/Game/Blueprints/Deck.InitializeDeck` _output_get_2 true)
  (`self.UserDrawCard`)
  (`self.AIDrawCard`)
  (`KismetSystemLibrary.Delay` _delayamount)
  (`self.UserDrawCard`)
  (`self.AIDrawCard`)
  (`KismetSystemLibrary.Delay` _delayamount)
  (`self.UserDrawCard`)
  (`self.AIDrawCard`)
  (`KismetSystemLibrary.Delay` _delayamount)
  (bind _asbattle_card_game_mode (cast `/Game/Blueprints/BattleCardGameMode` (`GameplayStatics.GetGameMode`)))
  (`/Game/Blueprints/BattleCardGameMode.TakeUserTurn` _asbattle_card_game_mode)
  (`self.UpdateIndicesAndPositions`))

(event `GetCardFromDeck`
  (params (Card :type "/Game/Blueprints/Card Object Reference") (Target :type "Vector Structure") (User :type Boolean))
  ;[1 1 1] Handle drawing from deck
  (if User
    (`/Game/Blueprints/Card.rotateCard` Card (struct :`Yaw` 180.0)))
  (`/Game/Blueprints/Card.moveCard` Card Target))

(event `UserDrawCard`
  (bind _deck1 (`self.Deck1`))
  (bind _handcards1 (`self.HandCards1`))
  (bind _handcount1 (`self.HandCount1`))
  ;[1 1 1] handle single card draw animation
  (bind _cardsremaining (`/Game/Blueprints/Deck.HasCardsLeft` (`self.Deck1`)))
  (if _cardsremaining
    (if (< (`KismetArrayLibrary.Array_Length` (`self.HandCards1`)) (`self.MaxHandSize`))
      (bind _nextcardid (`/Game/Blueprints/Deck.GetNextCardID` _deck1))
      (bind _returnvalue (`|SpawnActorFromClass` "/Game/Blueprints/Card.Card_C" (`KismetMathLibrary.MakeTransform` (+ (`self.DeckLocation1`) (0.0 0.0 35.0)) (struct :`Pitch` 180.0)) "Undefined" "OverrideRootScale"))
      (bind _returnvalue_2 (`KismetArrayLibrary.Array_Add` _handcards1 _returnvalue))
      (bind _item (`KismetArrayLibrary.Array_Get` _handcards1 _returnvalue_2))
      (`/Game/Blueprints/Card.ModifyText` _item _nextcardid)
      (`/Game/Blueprints/Card.SetIndex` _item _handcount1)
      (`self.GetCardFromDeck` _item (`KismetArrayLibrary.Array_Get` (`self.HandLocations1`) _handcount1) true)
      (`/Engine/EditorBlueprintResources/StandardMacros.IncrementInt` _handcount1
        (:`  `
          (`/Game/Blueprints/Deck.DecreaseCardCount` _deck1)))
      (else
        (`KismetSystemLibrary.PrintString` "Hand is Full")))
    (else
      (`KismetSystemLibrary.PrintString` "Deck is empty"))))

(event `AIDrawCard`
  (bind _deck2 (`self.Deck2`))
  (bind _handcards2 (`self.HandCards2`))
  (bind _handcount2 (`self.HandCount2`))
  ;[1 1 1] handle single card draw animation
  (bind _cardsremaining (`/Game/Blueprints/Deck.HasCardsLeft` (`self.Deck2`)))
  (if _cardsremaining
    (if (< (`KismetArrayLibrary.Array_Length` (`self.HandCards2`)) (`self.MaxHandSize`))
      (bind _nextcardid (`/Game/Blueprints/Deck.GetNextCardID` _deck2))
      (bind _returnvalue (`|SpawnActorFromClass` "/Game/Blueprints/Card.Card_C" (`KismetMathLibrary.MakeTransform` (+ (`self.DeckLocation2`) (0.0 0.0 35.0)) (struct :`Pitch` 180.0)) "Undefined" "OverrideRootScale"))
      (set `/Game/Blueprints/Card.UserOwned` false _returnvalue)
      (bind _returnvalue_2 (`KismetArrayLibrary.Array_Add` _handcards2 _returnvalue))
      (bind _item (`KismetArrayLibrary.Array_Get` _handcards2 _returnvalue_2))
      (`/Game/Blueprints/Card.ModifyText` _item _nextcardid)
      (`/Game/Blueprints/Card.SetIndex` _item _handcount2)
      (`self.GetCardFromDeck` _item (`KismetArrayLibrary.Array_Get` (`self.HandLocations2`) _handcount2))
      (`/Engine/EditorBlueprintResources/StandardMacros.IncrementInt` _handcount2
        (:`  `
          (`/Game/Blueprints/Deck.DecreaseCardCount` _deck2)))
      (else
        (`KismetSystemLibrary.PrintString` "Hand is Full")))))

(event `UserPlayCardFromHand`
  (params (Index :type Integer))
  (bind _handcards1 (`self.HandCards1`))
  (bind _boardcards1 (`self.BoardCards1`))
  (bind _boardcount1 (`self.BoardCount1`))
  (bind _item (`KismetArrayLibrary.Array_Get` _handcards1 Index))
  ;[1 1 1] Handle basic hand to board mechanic
  (bind _havemana (`self.CheckForSufficientMana` Index true))
  (if _havemana
    (if (< (`self.BoardCount1`) 6)
      (`/Game/Blueprints/Card.moveCard` _item (`KismetArrayLibrary.Array_Get` (`self.BoardLocations1`) _boardcount1))
      (`/Engine/EditorBlueprintResources/StandardMacros.IncrementInt` _boardcount1
        (:`  `
          (bind _returnvalue (`KismetArrayLibrary.Array_Add` _boardcards1 _item))
          (`KismetArrayLibrary.Array_Remove` _handcards1 Index)
          (bind _item_2 (`KismetArrayLibrary.Array_Get` _boardcards1 _returnvalue))
          (set `/Game/Blueprints/Card.InHand` false _item_2)
          (`self.UpdateIndicesAndPositions`)
          (`/Engine/EditorBlueprintResources/StandardMacros.DecrementInt` (`self.HandCount1`)
            (:`  `
              (`/Engine/EditorBlueprintResources/StandardMacros.IncrementInt` (`/Game/Blueprints/Card.SummonCounter` _item_2))))))
      (else
        (`KismetSystemLibrary.PrintString` "Board Full")
        (`/Game/Blueprints/Card.moveCard` (`KismetArrayLibrary.Array_Get` (`self.HandCards1`) Index) (`KismetArrayLibrary.Array_Get` (`self.HandLocations1`) Index) :!label _label)))
    (else
      (`KismetSystemLibrary.PrintString` "Not Enough Mana")
      (goto _label))))

(event `AIPlayCardFromHand`
  (params (Index :type Integer))
  (bind _boardcount2 (`self.BoardCount2`))
  (bind _boardcards2 (`self.BoardCards2`))
  (bind _handcards2 (`self.HandCards2`))
  (bind _item (`KismetArrayLibrary.Array_Get` (`self.HandCards2`) Index))
  (bind _item_2 (`KismetArrayLibrary.Array_Get` _handcards2 Index))
  ;[1 1 1] Handle basic hand to board mechanic
  (bind _havemana (`self.CheckForSufficientMana` Index))
  (if _havemana
    (if (< (`self.BoardCount2`) 6)
      (`/Game/Blueprints/Card.moveCard` _item_2 (+ (`KismetArrayLibrary.Array_Get` (`self.HandLocations2`) Index) (0.0 0.0 20.0)))
      (`/Game/Blueprints/Card.moveCard` _item_2 (`KismetArrayLibrary.Array_Get` (`self.BoardLocations2`) _boardcount2))
      (`/Game/Blueprints/Card.rotateCard` _item_2 (struct :`Yaw` 180.0))
      (`/Engine/EditorBlueprintResources/StandardMacros.IncrementInt` _boardcount2
        (:`  `
          (bind _returnvalue (`KismetArrayLibrary.Array_Add` _boardcards2 _item_2))
          (`KismetArrayLibrary.Array_Remove` _handcards2 Index)
          (set `/Game/Blueprints/Card.InHand` false (`KismetArrayLibrary.Array_Get` _boardcards2 _returnvalue))
          (`self.UpdateIndicesAndPositions`)
          (`/Engine/EditorBlueprintResources/StandardMacros.DecrementInt` (`self.HandCount2`))))
      (else
        (`KismetSystemLibrary.PrintString` "Board Full")
        (`/Game/Blueprints/Card.moveCard` _item (`KismetArrayLibrary.Array_Get` (`self.HandLocations2`) Index) :!label _label_2)
        (`/Game/Blueprints/Card.rotateCard` _item (struct :`Yaw` 180.0))))
    (else
      (goto _label_2))))

(event `PlayButtonPressed`
  ;[1 1 1] Check for play button before playing cards
  (`/Engine/EditorBlueprintResources/StandardMacros.Gate` true :!label _label_3
    (:`Exit`
      (if (stale `AnyCardClicked` InHand)
        (`self.UserPlayCardFromHand` (stale `AnyCardClicked` Index))
        (set `self.HaveActiveCard` false)
        (set `self.ClickCount` 0)
        (goto _label_3 :!via `Close`)
        (else
          (set `self.HaveActiveCard` false :!label _label_4)
          (bind _newparam (`self.GetCardLocation` (stale `AnyCardClicked` User) (stale `AnyCardClicked` InHand) (stale `AnyCardClicked` Index)))
          (`/Game/Blueprints/Card.moveCard` (stale `AnyCardClicked` _item) _newparam)
          (set `self.ClickCount` 0)
          (`self.DeclineCombat`)
          (goto _label_3 :!via `Close`))))))

(event `RemoveFromBoard`
  (params (Index :type Integer))
  ;[1 1 1] Temporary Board Card Removal
  (`KismetArrayLibrary.Array_Remove` (`self.BoardCards1`) Index)
  (`self.UpdateIndicesAndPositions`)
  (`/Engine/EditorBlueprintResources/StandardMacros.DecrementInt` (`self.BoardCount1`)))

(event `AnyCardClicked`
  (params (Index :type Integer) (InHand :type Boolean) (User :type Boolean))
  ;[1 1 1] Check for play button before playing cards
  (set `self.ActiveCardInHand` InHand)
  (set `self.ActiveCardUserOwned` User)
  (if (not (`self.HaveActiveCard`))
    (bind _item (`self.GetCardReference` InHand Index User))
    (`self.StartCombatCheck` _item)
    (set `self.HaveActiveCard` true)
    (set `self.ActiveCardIndex` Index)
    (bind _location (`/Game/Blueprints/Card.GetLocation` _item))
    (`/Game/Blueprints/Card.moveCard` _item (+ _location (0.0 0.0 10.0)))
    (`/Engine/EditorBlueprintResources/StandardMacros.IncrementInt` (`self.ClickCount`)
      (:`  `
        (goto _label_3 :!via `Open`)))
    (else
      ;;[1 1 1] if true, call zoom
      (if (< (`self.ClickCount`) 2)
        (`/Game/Blueprints/Card.ZoomCard` _item)
        (`/Engine/EditorBlueprintResources/StandardMacros.IncrementInt` (`self.ClickCount`))
        (else
          (goto _label_4))))))

(event `InitiateCombat`
  (params (Card2 :type "/Game/Blueprints/Card Object Reference"))
  ;[1 1 1] User attack mechanic
  (bind _output_get (set `self.CombatCard2` Card2))
  (`/Engine/EditorBlueprintResources/StandardMacros.Gate` true :!label _label_5
    (:`Exit`
      (if (not (`/Game/Blueprints/Card.HasAttacked` (stale `StartCombatCheck` _output_get)))
        (set `self.HaveActiveCard` false)
        (set `self.ClickCount` 0)
        (set `/Game/Blueprints/Card.HasAttacked` true (stale `StartCombatCheck` _output_get))
        (`self.CardCombatAnimation` (stale `StartCombatCheck` _output_get) _output_get true)
        (`KismetSystemLibrary.Delay` 1.5)
        (`self.CardCombat` (stale `StartCombatCheck` _output_get) _output_get)
        (else
          (if (> (`/Game/Blueprints/Card.SummonCounter` (stale `StartCombatCheck` _output_get)) 1)
            (`KismetSystemLibrary.PrintString` "That card already attacked")
            (else
              (`KismetSystemLibrary.PrintString` "Give that card a turn to get ready")))
          (set `self.HaveActiveCard` false)
          (set `self.ClickCount` 0)
          (`self.UpdateIndicesAndPositions`))))))

(event `StartCombatCheck`
  (params (Card1 :type "/Game/Blueprints/Card Object Reference"))
  ;[1 1 1] User attack mechanic
  (bind _output_get (set `self.CombatCard1` Card1))
  (goto _label_5 :!via `Open`))

(event `DeclineCombat`
  ;[1 1 1] User attack mechanic
  (goto _label_5 :!via `Close`))

(event `AITakeTurn`
  (bind _usercharacter (`self.UserCharacter`))
  (bind _aiboardindex (`self.AIBoardIndex`))
  (bind _item (`KismetArrayLibrary.Array_Get` (`self.BoardCards2`) _aiboardindex))
  ;[1 1 1] AI Turn
  (set `self.AIBoardIndex` 0)
  (if (> (`KismetArrayLibrary.Array_Length` (`self.BoardCards2`)) 0)
    (if (< _aiboardindex (`KismetArrayLibrary.Array_Length` (`self.BoardCards2`))) :!label _label_6
      (`self.CardCombatAnimation` _item _usercharacter)
      (`KismetSystemLibrary.Delay` 1.5)
      (`self.CardCombat` _item _usercharacter)
      (`/Engine/EditorBlueprintResources/StandardMacros.IncrementInt` (`self.AIBoardIndex`)
        (:`  `
          (goto _label_6)))
      (elif (not (> (`KismetArrayLibrary.Array_Length` (`self.BoardCards2`)) 5))
        (for (_ _array_index) (`self.HandCards2`) :!label _label_7
          (`self.AIPlayCardFromHand` _array_index))
        (bind _asbattle_card_game_mode (cast `/Game/Blueprints/BattleCardGameMode` (`GameplayStatics.GetGameMode`)))))
    (else
      (goto _label_7)))
  (`/Game/Blueprints/BattleCardGameMode.TakeUserTurn` _asbattle_card_game_mode))

(event `CardCombatAnimation`
  (params (AttackingCard :type "/Game/Blueprints/Card Object Reference") (DefendingCard :type "/Game/Blueprints/Card Object Reference") (UserAttacking :type Boolean))
  (bind _userowned (`/Game/Blueprints/Card.UserOwned` DefendingCard))
  (bind _index (`/Game/Blueprints/Card.Index` DefendingCard))
  ;[1 1 1] Ok, I need to add movement back to board location and fix AI Character combat interaction
  (if _userowned
    (if (`/Game/Blueprints/Card.IsCharacter` DefendingCard)
      (`/Game/Blueprints/Card.moveCard` AttackingCard (+ (`self.CharacterLocation1`) (`self.AIAttackMod`)))
      (else
        (`/Game/Blueprints/Card.moveCard` AttackingCard (+ (`KismetArrayLibrary.Array_Get` (`self.BoardLocations1`) _index) (`self.AIAttackMod`)))))
    (elif (`/Game/Blueprints/Card.IsCharacter` DefendingCard)
      (`/Game/Blueprints/Card.moveCard` AttackingCard (+ (`self.CharacterLocation2`) (`self.UserAttackMod`)))
      (else
        (`/Game/Blueprints/Card.moveCard` AttackingCard (+ (`KismetArrayLibrary.Array_Get` (`self.BoardLocations2`) _index) (`self.UserAttackMod`))))))
  (`KismetSystemLibrary.Delay` 0.8)
  (if _userowned
    (`/Game/Blueprints/Card.moveCard` AttackingCard (`KismetArrayLibrary.Array_Get` (`self.BoardLocations2`) (`/Game/Blueprints/Card.Index` AttackingCard)))
    (else
      (`/Game/Blueprints/Card.moveCard` AttackingCard (`KismetArrayLibrary.Array_Get` (`self.BoardLocations1`) (`/Game/Blueprints/Card.Index` AttackingCard))))))

(fn `ActiveCardCheck`
  (returns (Active :type Boolean) (Index :type Integer) (ActiveCardInHand :type Boolean) (ActiveCardUserOwned :type Boolean))
  (return (`self.HaveActiveCard`) (`self.ActiveCardIndex`) (`self.ActiveCardInHand`) (`self.ActiveCardUserOwned`)))

(fn `AddMana`
  (params (Amount :type Integer) (User :type Boolean))
  (if User
    (bind _output_get (set `self.UserMana` (+ Amount (`self.UserMana`))))
    (bind _outactors (`GameplayStatics.GetAllActorsOfClass` "/Game/Blueprints/ManaBall.ManaBall_C"))
    (bind _asmana_ball (cast `/Game/Blueprints/ManaBall` (`KismetArrayLibrary.Array_Get` _outactors)))
    (`/Game/Blueprints/ManaBall.SetManaText` _asmana_ball _output_get)
    (else
      (set `self.AIMana` (+ Amount (`self.AIMana`))))))

(fn `CardCombat`
  (params (AttackingCard :type "/Game/Blueprints/Card Object Reference") (DefendingCard :type "/Game/Blueprints/Card Object Reference"))
  (locals (ACard :type "/Game/Blueprints/Card Object Reference") (DCard :type "/Game/Blueprints/Card Object Reference") (power1 :type Integer) (power2 :type Integer))
  (bind _acard (`local.ACard`))
  (bind _dcard (`local.DCard`))
  (bind _returnvalue (- (`local.power2`) (`local.power1`)))
  (bind _returnvalue_2 (- (`local.power1`) (`local.power2`)))
  (set `local.ACard` AttackingCard)
  (set `local.DCard` DefendingCard)
  (bind _ascard (cast `/Game/Blueprints/Card` AttackingCard))
  (bind (_cardid _name _cost _iscreature _power _cardeffect _effectvalue _dealscombatdamage) (break `/Game/Data/CardDataStruct` (`/Game/Blueprints/Card.CardData` _ascard)))
  (if _dealscombatdamage
    (bind _ascard_2 (cast `/Game/Blueprints/Card` DefendingCard))
    (set `local.power1` _power)
    (bind (_cardid_2 _name_2 _cost_2 _iscreature_2 _power_2 _cardeffect_2 _effectvalue_2 _dealscombatdamage_2) (break `/Game/Data/CardDataStruct` (`/Game/Blueprints/Card.CardData` _ascard_2)))
    (set `local.power2` _power_2)
    (if _dealscombatdamage_2
      (if (> _returnvalue_2 0)
        (`/Game/Blueprints/Card.SetPower` _acard _returnvalue_2)
        (if (> _returnvalue 0) :!label _label
          (`/Game/Blueprints/Card.SetPower` _dcard _returnvalue)
          (else
            (`/Game/Blueprints/Card.SetPower` _dcard 0)
            (bind _ascard_3 (cast `/Game/Blueprints/Card` (`local.DCard`)))
            (if (`/Game/Blueprints/Card.IsCharacter` _ascard_3)
              _
              (elif (`/Game/Blueprints/Card.UserOwned` _ascard_3)
                (bind _index (`/Game/Blueprints/Card.Index` _ascard_3))
                (`KismetArrayLibrary.Array_Remove` (`self.BoardCards1`) _index)
                (`self.K2_DestroyActor` (`local.DCard`))
                (`self.UpdateIndicesAndPositions`)
                (set `self.HaveActiveCard` false)
                (set `self.ClickCount` 0)
                (`/Engine/EditorBlueprintResources/StandardMacros.DecrementInt` (`self.BoardCount1`))
                (else
                  (`KismetArrayLibrary.Array_Remove` (`self.BoardCards2`) _index)
                  (`self.K2_DestroyActor` (`local.DCard`))
                  (`self.UpdateIndicesAndPositions`)
                  (set `self.HaveActiveCard` false)
                  (set `self.ClickCount` 0)
                  (`/Engine/EditorBlueprintResources/StandardMacros.DecrementInt` (`self.BoardCount2`)))))))
        (else
          (`/Game/Blueprints/Card.SetPower` _acard 0)
          (bind _ascard_4 (cast `/Game/Blueprints/Card` (`local.ACard`)))
          (if (`/Game/Blueprints/Card.IsCharacter` _ascard_4)
            _
            (elif (`/Game/Blueprints/Card.UserOwned` _ascard_4)
              (bind _index_2 (`/Game/Blueprints/Card.Index` _ascard_4))
              (`KismetArrayLibrary.Array_Remove` (`self.BoardCards1`) _index_2)
              (`self.K2_DestroyActor` (`local.ACard`))
              (`self.UpdateIndicesAndPositions`)
              (set `self.HaveActiveCard` false)
              (set `self.ClickCount` 0)
              (`/Engine/EditorBlueprintResources/StandardMacros.DecrementInt` (`self.BoardCount1`)
                (:`  `
                  (goto _label)))
              (else
                (`KismetArrayLibrary.Array_Remove` (`self.BoardCards2`) _index_2)
                (`self.K2_DestroyActor` (`local.ACard`))
                (`self.UpdateIndicesAndPositions`)
                (set `self.HaveActiveCard` false)
                (set `self.ClickCount` 0)
                (`/Engine/EditorBlueprintResources/StandardMacros.DecrementInt` (`self.BoardCount2`)
                  (:`  `
                    (goto _label))))))))
      (else
        (goto _label)))
    (else
      (`KismetSystemLibrary.PrintString` "That card can't attack"))))

(fn `CheckForSufficientMana`
  (params (CardIndex :type Integer) (User :type Boolean))
  (returns (HaveMana :type Boolean))
  (if User
    (bind _manacost (`/Game/Blueprints/Card.GetManaCost` (`KismetArrayLibrary.Array_Get` (`self.HandCards1`) CardIndex)))
    (if (>= (`self.UserMana`) _manacost)
      (`self.SubtractMana` _manacost true)
      (return true)
      (else
        (return false)))
    (else
      (bind _manacost_2 (`/Game/Blueprints/Card.GetManaCost` (`KismetArrayLibrary.Array_Get` (`self.HandCards2`) CardIndex)))
      (if (>= (`self.AIMana`) _manacost_2)
        (`self.SubtractMana` _manacost_2)
        (return true)
        (else
          (return false))))))

(fn `GetCardLocation`
  (params (User :type Boolean) (InHand :type Boolean) (Index :type Integer))
  (returns (NewParam :type "Vector Structure"))
  (if User
    (if InHand
      (return (`KismetArrayLibrary.Array_Get` (`self.HandLocations1`) Index))
      (else
        (return (`KismetArrayLibrary.Array_Get` (`self.BoardLocations1`) Index))))
    (elif InHand
      (return (`KismetArrayLibrary.Array_Get` (`self.HandLocations2`) Index))
      (else
        (return (`KismetArrayLibrary.Array_Get` (`self.BoardLocations2`) Index))))))

(fn `GetCardReference`
  (params (InHand :type Boolean) (Index :type Integer) (UserOwned :type Boolean))
  (returns (Item :type "/Game/Blueprints/Card Object Reference"))
  (if UserOwned
    (if InHand
      (return (`KismetArrayLibrary.Array_Get` (`self.HandCards1`) Index))
      (else
        (return (`KismetArrayLibrary.Array_Get` (`self.BoardCards1`) Index))))
    (elif InHand
      (return (`KismetArrayLibrary.Array_Get` (`self.HandCards2`) Index))
      (else
        (return (`KismetArrayLibrary.Array_Get` (`self.BoardCards2`) Index))))))

(fn `SubtractMana`
  (params (Amount :type Integer) (User :type Boolean))
  (if User
    (bind _output_get (set `self.UserMana` (- (`self.UserMana`) Amount)))
    (bind _outactors (`GameplayStatics.GetAllActorsOfClass` "/Game/Blueprints/ManaBall.ManaBall_C"))
    (bind _asmana_ball (cast `/Game/Blueprints/ManaBall` (`KismetArrayLibrary.Array_Get` _outactors)))
    (`/Game/Blueprints/ManaBall.SetManaText` _asmana_ball _output_get)
    (else
      (set `self.AIMana` (- (`self.AIMana`) Amount)))))

(fn `UpdateIndicesAndPositions`
  (for (_array_element _array_index) (`self.HandCards1`)
    (`/Game/Blueprints/Card.SetIndex` _array_element _array_index)
    (`/Game/Blueprints/Card.moveCard` _array_element (`KismetArrayLibrary.Array_Get` (`self.HandLocations1`) _array_index)))
  (for (_array_element_2 _array_index_2) (`self.BoardCards1`)
    (`/Game/Blueprints/Card.SetIndex` _array_element_2 _array_index_2)
    (`/Game/Blueprints/Card.moveCard` _array_element_2 (`KismetArrayLibrary.Array_Get` (`self.BoardLocations1`) _array_index_2)))
  (for (_array_element_3 _array_index_3) (`self.HandCards2`)
    (`/Game/Blueprints/Card.SetIndex` _array_element_3 _array_index_3)
    (`/Game/Blueprints/Card.moveCard` _array_element_3 (`KismetArrayLibrary.Array_Get` (`self.HandLocations2`) _array_index_3)))
  (for (_array_element_4 _array_index_4) (`self.BoardCards2`)
    (`/Game/Blueprints/Card.SetIndex` _array_element_4 _array_index_4)
    (`/Game/Blueprints/Card.moveCard` _array_element_4 (`KismetArrayLibrary.Array_Get` (`self.BoardLocations2`) _array_index_4))))

(fn `UserConstructionScript`)