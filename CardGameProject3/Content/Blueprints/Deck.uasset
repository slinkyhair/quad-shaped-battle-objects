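; Card deck for a battle card game that holds a shuffled list of card IDs and requests a user draw when its mesh is clicked.
; InitializeDeck builds 30 cards, all one ID for the AI or an even mix of five IDs for the user.
; GetNextCardID walks the list on authority, returning -1 when exhausted, while a separate counter tracks cards left.
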(event `DecreaseCardCount`
  (`/Engine/EditorBlueprintResources/StandardMacros.DecrementInt` (`self.NumCardsLeft`)))

(event `self.StaticMeshComponent.OnClicked`
  (params (TouchedComponent :type "PrimitiveComponent Object Reference") (ButtonPressed :type "Key Structure" :default "AnyKey"))
  (bind _asbattle_card_game_state (cast `/Game/Blueprints/BattleCardGameState` (`GameplayStatics.GetGameState`)))
  (`/Game/Blueprints/BattleCardGameState.UserDrawCard` _asbattle_card_game_state))

(event `InitializeDeck`
  (params (AI :type Boolean))
  ;[1 1 1] Initialize User and AI Decks
  (if AI
    (for _ (range 1 31)
      (`KismetArrayLibrary.Array_Add` (`self.DeckList`) 1)
      (`KismetArrayLibrary.Array_Shuffle` (`self.DeckList`) :!label _label))
    (else
      (for _ (range 1 7)
        (`KismetArrayLibrary.Array_Add` (`self.DeckList`) 1))
      (for _ (range 1 7)
        (`KismetArrayLibrary.Array_Add` (`self.DeckList`) 2))
      (for _ (range 1 7)
        (`KismetArrayLibrary.Array_Add` (`self.DeckList`) 3))
      (for _ (range 1 7)
        (`KismetArrayLibrary.Array_Add` (`self.DeckList`) 4))
      (for _ (range 1 7)
        (`KismetArrayLibrary.Array_Add` (`self.DeckList`) 5))
      (goto _label))))

(fn `GetNextCardID`
  (returns (nextCardID :type Integer))
  (`/Engine/EditorBlueprintResources/ActorMacros.Switch Has Authority`
    (:`Authority`
      (if (< (`self.Iterator`) (`KismetArrayLibrary.Array_Length` (`self.DeckList`)))
        (bind _output_get (set `self.currentCardIndex` (`self.Iterator`)))
        (`/Engine/EditorBlueprintResources/StandardMacros.IncrementInt` (`self.Iterator`)
          (:`  `
            (return (`KismetArrayLibrary.Array_Get` (`self.DeckList`) _output_get))))
        (else
          (return -1))))))

(fn `HasCardsLeft`
  (returns (CardsRemaining :type Boolean))
  (return (> (`self.NumCardsLeft`) 0)))

(fn `UserConstructionScript`)