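; A clickable End Turn button actor for a card battle game.
; Clicking its static mesh nudges the actor down and, after a brief delay, back up to mimic a button press.
; It then asks BattleCardGameMode to take the user's turn, but only if BattleCardGameState reports no active card.
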(event `self.StaticMeshComponent.OnClicked`
  (params (TouchedComponent :type "PrimitiveComponent Object Reference") (ButtonPressed :type "Key Structure" :default "AnyKey"))
  (`self.K2_SetActorRelativeLocation` (+ (`self.K2_GetActorLocation`) (0.0 0.0 -2.0)))
  (`KismetSystemLibrary.Delay` 0.09)
  (`self.K2_SetActorRelativeLocation` (+ (`self.K2_GetActorLocation`) (0.0 0.0 2.0)))
  (bind _asbattle_card_game_mode (cast `/Game/Blueprints/BattleCardGameMode` (`GameplayStatics.GetGameMode`)))
  (bind _asbattle_card_game_state (cast `/Game/Blueprints/BattleCardGameState` (`GameplayStatics.GetGameState`)))
  (if (not (`/Game/Blueprints/BattleCardGameState.HaveActiveCard` _asbattle_card_game_state))
    (`/Game/Blueprints/BattleCardGameMode.TakeUserTurn` _asbattle_card_game_mode)))

(fn `UserConstructionScript`)